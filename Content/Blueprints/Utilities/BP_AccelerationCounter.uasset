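; BP_AccelerationCounter is a debug utility that measures how long a Racecar takes to accelerate from standstill to a target Speed in km/h.
; Tick accumulates elapsed time while the car moves and resets the timer whenever its speed is exactly zero.
; Reaching the target prints the car's name and time on screen once per run.
; An invalid Racecar reference logs an error instead.
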(event `self.ReceiveBeginPlay`
  ;[0.08333 0.08333 0.08333] Initialise and Preliminary Checks
  (`parent.ReceiveBeginPlay`)
  (set `self.TimeTaken` 0.0))

(event `self.ReceiveTick`
  (params (DeltaSeconds :type "Float (single-precision)"))
  (bind _returnvalue (`Racecar.GetSpeed` (`self.Racecar`)))
  (if (`KismetSystemLibrary.IsValid` (`self.Racecar`))
    (if (== _returnvalue 0)
      (set `self.TimeTaken` 0.0)
      (set `self.bHasShownOnScreen` false)
      (else
        (set `self.TimeTaken` (+ DeltaSeconds (`self.TimeTaken`)))
        (if (and (>= _returnvalue (`self.Speed`)) (not (`self.bHasShownOnScreen`)))
          (`KismetSystemLibrary.PrintText` (`|FormatText` "{Racecar}:0-{Speed} km/h in {Time} seconds." (`self.Speed`) (`self.TimeTaken`) (`KismetSystemLibrary.GetDisplayName` (`self.Racecar`))) true false (struct :`R` 1.0 :`G` 0.970537 :`B` 0.992634 :`A` 1.0) 4.0)
          (set `self.bHasShownOnScreen` true))))
    (else
      (`KismetSystemLibrary.PrintText` (`|FormatText` "{0} Racecar is nullptr." (`self.GetOwner`)) false true (struct :`R` 1.0 :`G` 0.101111 :`A` 1.0)))))