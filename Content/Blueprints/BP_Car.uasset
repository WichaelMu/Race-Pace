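; BP_Car is a player-drivable car Blueprint controlled through its VehicleMovement component.
; Throttle, Brake and Steer axis inputs pass straight into the component's throttle, brake and steering inputs.
; Tick prints the engine rotation speed to screen every frame as a debug readout.
; BeginPlay and the construction script are empty.
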(event `self.ReceiveTick`
  (params (DeltaSeconds :type "Float (single-precision)"))
  (`KismetSystemLibrary.PrintString` (`KismetStringLibrary.Conv_DoubleToString` (`WheeledVehicleMovementComponent.GetEngineRotationSpeed` (`self.VehicleMovement`))) true false))

(event `InputAxis|Throttle`
  (params (AxisValue :type "Float (single-precision)"))
  (`WheeledVehicleMovementComponent.SetThrottleInput` (`self.VehicleMovement`) AxisValue))

(event `InputAxis|Brake`
  (params (AxisValue :type "Float (single-precision)"))
  (`WheeledVehicleMovementComponent.SetBrakeInput` (`self.VehicleMovement`) AxisValue))

(event `InputAxis|Steer`
  (params (AxisValue :type "Float (single-precision)"))
  (`WheeledVehicleMovementComponent.SetSteeringInput` (`self.VehicleMovement`) AxisValue))

(fn `UserConstructionScript`)